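; BP_PatrolPoints is a spline-based patrol route actor that supplies waypoint positions, presumably for patrolling AI.
; GetNextSplinPoint steps CurrentIndex by Diraction and flips the direction at the first and last spline points, giving a ping-pong route.
; GetSplinPointPOS returns the world location of the current point.
; The event graph and construction script are empty, so the route only changes when these functions are called.
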(event EventBeginPlay)

(event Collision|EventActorBeginOverlap
  (params (OtherActor :type Actor%20Object%20Reference)))

(event EventTick
  (params (DeltaSeconds :type Float%20%28single-precision%29)))

(fn ConstructionScript)

(fn GetNextSplinPoint
  (bind _output_get (Variables|Default|SetCurrentIndex (+ (Variables|Default|GetCurrentIndex) (Variables|Default|GetDiraction))))
  (if (== _output_get (- (Spline|GetNumberOfSplinePoints (Variables|Default|GetSpline)) 1))
    (Variables|Default|SetDiraction -1)
    (elif (== (Variables|Default|GetCurrentIndex) 0)
      (Variables|Default|SetDiraction 1))))

(fn GetSplinPointPOS
  (return (Spline|GetLocationatSplinePoint (Variables|Default|GetSpline) (Variables|Default|GetCurrentIndex) "World")))