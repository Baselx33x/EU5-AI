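; BP_NPC_2_Melee is a melee NPC character Blueprint that builds on a parent class to handle attacking and weapon wielding.
; Attacking plays the NPC_Attack montage on the mesh and calls ONAttackMontageFinished when it completes or is interrupted.
; Two wield events share one path that spawns BP_Weaopen, snaps it to the right-hand socket and flags the NPC as armed.
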(event EventBeginPlay
  (|CallParentFunction))

(event Collision|EventActorBeginOverlap
  (params (OtherActor :type Actor%20Object%20Reference))
  (|CallParentFunction OtherActor) ; This node is disabled and will not be called.\nDrag off pins to build functionality.
)

(event EventTick
  (params (DeltaSeconds :type Float%20%28single-precision%29))
  (|CallParentFunction DeltaSeconds) ; This node is disabled and will not be called.\nDrag off pins to build functionality.
)

(event EventAttacking
  (Animation|Montage|PlayMontage (Variables|Character|GetMesh) "/Game/Secne_Two/AI/Tasks/NPC_Attack.NPC_Attack"
    (:OnCompleted
      _)
    (:OnInterrupted
      _))
  (Default|CallONAttackMontageFinished))

(event EventWieldWeaopen
  (bind _returnvalue (Game|SpawnActorfromClass "/Game/Secne_Two/BluePrints/BP_Weaopen.BP_Weaopen_C" (Transformation|GetActorTransform) "Undefined" "MultiplyWithRoot" 0 0))
  (Transformation|AttachComponentToComponent _returnvalue (Variables|Character|GetMesh) "hand_rSocket" "SnapToTarget" "SnapToTarget" "SnapToTarget" true)
  (Variables|Default|SetIsWieldingWeapon true))

(event EventWeildWeaopenfromMainClass
  (bind _returnvalue (Game|SpawnActorfromClass "/Game/Secne_Two/BluePrints/BP_Weaopen.BP_Weaopen_C" (Transformation|GetActorTransform) "Undefined" "MultiplyWithRoot" 0 0))
  (Transformation|AttachComponentToComponent _returnvalue (Variables|Character|GetMesh) "hand_rSocket" "SnapToTarget" "SnapToTarget" "SnapToTarget" true)
  (Variables|Default|SetIsWieldingWeapon true))

(fn ConstructionScript
  (|CallParentFunction))