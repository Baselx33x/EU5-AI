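; Shooting enemy NPC, a child Blueprint that overrides weapon and attack events.
; Wielding spawns a BP_Weaopen, snaps it to the hand socket and flags it as wielded.
; ShootGun plays a shooting montage, with a notify triggering a debug-drawn Visibility trace toward the player that stores any hit as DidHitPlayer.
; Montage completion or interruption signals attack finished; Attacking is empty and no damage is applied here.
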(event EventBeginPlay
  (|CallParentFunction))

(event Collision|EventActorBeginOverlap
  (params (OtherActor :type Actor%20Object%20Reference))
  (|CallParentFunction OtherActor) ; This node is disabled and will not be called.\nDrag off pins to build functionality.
)

(event EventTick
  (params (DeltaSeconds :type Float%20%28single-precision%29))
  (|CallParentFunction DeltaSeconds) ; This node is disabled and will not be called.\nDrag off pins to build functionality.
)

(event EventAttacking)

(event EventShootGun
  (bind _notifyname (Animation|Montage|PlayMontage (Variables|Character|GetMesh) "/Game/Secne_Two/AI/Tasks/NPC_ShootingGun.NPC_ShootingGun")
    (:OnCompleted
      (Default|CallONAttackMontageFinished :!label _label))
    (:OnInterrupted
      (goto _label))
    (:OnNotifyBegin
      (switch name _notifyname
        (:ShootGun
          (bind _returnvalue (Collision|LineTraceByChannel (+ (Transformation|GetActorLocation) (* "0.000000,0.000000,1.000000" "0.000000,0.000000,75.000000")) (Transformation|GetActorLocation (Game|GetPlayerCharacter 0)) "TraceTypeQuery1" false 0 "ForDuration"))
          (Variables|Default|SetDidHitPlayer%20? _returnvalue))))))

(event EventWieldWeaopen
  (bind _returnvalue (Game|SpawnActorfromClass "/Game/Secne_Two/BluePrints/BP_Weaopen.BP_Weaopen_C" (Transformation|GetActorTransform) "Undefined" "MultiplyWithRoot" 0 0))
  (Transformation|AttachComponentToComponent _returnvalue (Variables|Character|GetMesh) "hand_rSocket" "SnapToTarget" "SnapToTarget" "SnapToTarget" true)
  (Variables|Default|SetIsWieldingWeapon true))

(event EventWeildWeaopenfromMainClass
  (bind _returnvalue (Game|SpawnActorfromClass "/Game/Secne_Two/BluePrints/BP_Weaopen.BP_Weaopen_C" (Transformation|GetActorTransform) "Undefined" "MultiplyWithRoot" 0 0))
  (Transformation|AttachComponentToComponent _returnvalue (Variables|Character|GetMesh) "hand_rSocket" "SnapToTarget" "SnapToTarget" "SnapToTarget" true)
  (Variables|Default|SetIsWieldingWeapon true))

(fn ConstructionScript
  (|CallParentFunction))